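; Jetpack actor that shows exhaust effects and plays sound while its owning third-person character is in jetpack mode.
; Each tick it casts its parent actor to BP_ThirdPersonCharacter and reads the JetPackMode flag.
; A DoOnce starts the sound and reveals two particle systems once per activation; when the flag is off, it stops and hides them and resets the gate.
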(event `self.ReceiveTick`
  (params (DeltaSeconds :type "Float (single-precision)"))
  (bind _asbp_third_person_character (cast `/Game/ThirdPerson/Blueprints/BP_ThirdPersonCharacter` (`self.GetParentActor`)))
  (if (`/Game/ThirdPerson/Blueprints/BP_ThirdPersonCharacter.JetPackMode` _asbp_third_person_character)
    (`/Engine/EditorBlueprintResources/StandardMacros.DoOnce` false :!label _label
      (:`Completed`
        (`AudioComponent.Play` (`self.JetPackSound`) 0.0)
        (`SceneComponent.SetVisibility` (`self.ParticleSystem1`) true false)
        (`SceneComponent.SetVisibility` (`self.ParticleSystem`) true false)))
    (else
      (`|ExecutionSequence`
        (:`then_0`
          (`AudioComponent.Stop` (`self.JetPackSound`))
          (`SceneComponent.SetVisibility` (`self.ParticleSystem1`) false false)
          (`SceneComponent.SetVisibility` (`self.ParticleSystem`) false false))
        (:`then_1`
          (goto _label :!via `Reset`))))))

(fn `UserConstructionScript`)